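; RicardoBP is the Ricardo quest-giver NPC that opens his quest dialog when the player clicks or touches his skeletal mesh.
; Both inputs share one path that hides the TopDownCharacter's main and stats HUD, calls Quest1Ricardo on AllQuest_BP to show the dialog, then hides his widget.
; The path also checks Quest3Completed on Quest1_BP, leading only to an empty DoOnce.
; DestroyWidget removes the widget and sets a flag that guards later visibility changes.
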(event OnInputTouchBegin(SkeletalMeshComponent)
  (params (FingerIndex :type ETouchIndex%20Enum :default "Touch1") (TouchedComponent :type Primitive%20Component%20Object%20Reference))
  (bind _returnvalue (Actor|GetActorOfClass "/Game/TopDownBP/Blueprints/Quest1_BP.Quest1_BP_C"))
  (if (Variables|/Game/TopDownBP/Blueprints/Quest1_BP.Quest1_BP_C|GetQuest3Completed _returnvalue)
    (Utilities|FlowControl|DoOnce false
      (:Completed
        _)))
  (bind _astop_down_character (Utilities|Casting|CastToTopDownCharacter (Game|GetPlayerCharacter 0)))
  (Default|HudShowHide _astop_down_character false false)
  (bind _returnvalue_2 (Actor|GetActorOfClass "/Game/TopDownBP/Blueprints/AllQuest_BP.AllQuest_BP_C"))
  (Default|Quest1Ricardo _returnvalue_2 false true)
  (CallFunction|WidgetVisibility false))

(event OnClicked(SkeletalMeshComponent)
  (params (TouchedComponent :type Primitive%20Component%20Object%20Reference) (ButtonPressed :type Key%20Structure :default "None"))
  (bind _returnvalue (Actor|GetActorOfClass "/Game/TopDownBP/Blueprints/Quest1_BP.Quest1_BP_C"))
  (if (Variables|/Game/TopDownBP/Blueprints/Quest1_BP.Quest1_BP_C|GetQuest3Completed _returnvalue)
    (Utilities|FlowControl|DoOnce false
      (:Completed
        _)))
  (bind _astop_down_character (Utilities|Casting|CastToTopDownCharacter (Game|GetPlayerCharacter 0)))
  (Default|HudShowHide _astop_down_character false false)
  (bind _returnvalue_2 (Actor|GetActorOfClass "/Game/TopDownBP/Blueprints/AllQuest_BP.AllQuest_BP_C"))
  (Default|Quest1Ricardo _returnvalue_2 false true)
  (CallFunction|WidgetVisibility false))

(fn ConstructionScript)

(fn WidgetVisibility
  (params (Visible :type Boolean))
  (if (not (Variables|Default|GetWidgetDestoyed))
    (Rendering|SetVisibility (Variables|Default|GetWidget) Visible false)))

(fn DestroyWidget
  (Components|DestroyComponent (Variables|Default|GetWidget))
  (Variables|Default|SetWidgetDestoyed true))