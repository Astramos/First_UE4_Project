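; Moczar enemy character that melee-attacks, takes damage and awards experience to the player when killed.
; Tick updates a floating widget with its name and health.
; Attack halts movement and plays a montage until AttackEnded restores speed, while events toggle the hit collision.
; Do-once gates limit each swing to one overlap hit with randomized, possibly critical damage, and death destroys the actor after a short delay.
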(event OnComponentBeginOverlap(AttackCollision)
  (params (OverlappedComponent :type Primitive%20Component%20Object%20Reference) (OtherActor :type Actor%20Object%20Reference) (OtherComp :type Primitive%20Component%20Object%20Reference) (OtherBodyIndex :type Integer) (bFromSweep :type Boolean) (SweepResult :type Hit%20Result%20Structure%20%28by%20ref%29))
  (if (!= OtherActor self)
    (Utilities|FlowControl|DoOnce false
      (:Completed
        (Game|Damage|ApplyDamage 0 0.0 0 0)
        (if (Math|Random|RandomBoolwithWeight 0.3)
          (Game|Damage|ApplyDamage OtherActor (Math|Random|RandomFloatinRange 2e+02 225.0) 0 0)
          (else
            (Game|Damage|ApplyDamage OtherActor (Math|Random|RandomFloatinRange 1e+02 1.5e+02) 0 0)))))))

(event Custom|Attack
  (if (not (Variables|Default|GetIsDead?))
    (Utilities|FlowControl|DoOnce false
      (:Completed
        (Variables|/Script/Engine.CharacterMovementComponent|SetMaxWalkSpeed (Variables|Character|GetCharacterMovement) 0.0)
        (Animation|PlayAnimMontage "/Game/Enemys/Animation/AttackAM.AttackAM" 1.0 "None")))))

(event Custom|AttackEnded
  (Variables|/Script/Engine.CharacterMovementComponent|SetMaxWalkSpeed (Variables|Character|GetCharacterMovement) (Variables|Default|GetStart%20max%20speed))
  (Utilities|FlowControl|DoOnce false) ; enters at Reset
)

(event Custom|Enable%20Collision
  (Collision|SetCollisionEnabled (Variables|Default|GetAttackCollision) "QueryOnly")
  (Audio|PlaySound2D "/Game/Sounds/MoczarAttack.MoczarAttack" 0.5 1.0 0.0 0 0))

(event Custom|Disable%20Collision
  (Collision|SetCollisionEnabled (Variables|Default|GetAttackCollision) "NoCollision")
  (CallFunction|Refresh))

(event Custom|Refresh
  (Utilities|FlowControl|DoOnce false) ; enters at Reset
)

(event Custom|On%20Death
  (if (not (Variables|Default|GetIsDead?))
    (Variables|Default|SetIsDead? true)
    (bind _astop_down_character (Utilities|Casting|CastToTopDownCharacter (Game|GetPlayerCharacter 0)))
    (Default|AddExp (Variables|/Game/TopDownBP/Blueprints/TopDownCharacter.TopDownCharacter_C|GetLevelAndExp_BP _astop_down_character) (Variables|Default|GetExpForKill))
    (Utilities|FlowControl|Delay 0.2)
    (Actor|DestroyActor)))

(event EventBeginPlay
  ;[1 1 1] Create floating widget reference to edit
  (Variables|Default|SetHP_Bar_Reference (.AsHP%20Bar (Utilities|Casting|CastToHP_Bar (UserInterface|GetUserWidgetObject (Variables|Default|GetHP_Bar)))))
  (Variables|Default|SetStart%20max%20speed (Variables|/Script/Engine.CharacterMovementComponent|GetMaxWalkSpeed (Variables|Character|GetCharacterMovement))))

(event Game|Damage|EventAnyDamage
  (params (Damage :type Float%20%28single-precision%29) (DamageType :type Damage%20Type%20Object%20Reference) (InstigatedBy :type Controller%20Object%20Reference) (DamageCauser :type Actor%20Object%20Reference))
  ;[1 1 1] Get damage
  (Variables|Default|SetCurrentHP (- (Variables|Default|GetCurrentHP) Damage))
  (if (<= (Variables|Default|GetCurrentHP) 0.0)
    (CallFunction|OnDeath)))

(event EventTick
  (params (DeltaSeconds :type Float%20%28single-precision%29))
  (bind _hp_bar_reference (Variables|Default|GetHP_Bar_Reference))
  ;[1 1 1] Show stats on widget
  (Progress|SetPercent (Variables|/Game/UI/Enemy/HP_Bar.HP_Bar_C|GetEnemyProgressBar _hp_bar_reference) (Math|Float|NormalizetoRange (Variables|Default|GetCurrentHP) 0.0 (Variables|Default|GetMaxHP)))
  (Rendering|Components|TextRender|SetText (Variables|/Game/UI/Enemy/HP_Bar.HP_Bar_C|GetEnemyName _hp_bar_reference) (Utilities|Text|ToText(Name) (Variables|Default|GetName))))

(fn ConstructionScript)